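; B3HUD is a HUD Blueprint that draws a simple white crosshair at the center of the screen.
; Each DrawHUD call draws two thin rectangles, one horizontal and one vertical, centered on half the viewport width and height.
; A fixed literal sets the arm length, and all other events and the construction script are empty.
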(event EventBeginPlay)

(event Collision|EventActorBeginOverlap
  (params (OtherActor :type Actor%20Object%20Reference)))

(event EventTick
  (params (DeltaSeconds :type Float%20%28single-precision%29)))

(event EventDrawHUD
  (params (SizeX :type Integer) (SizeY :type Integer))
  (bind _returnvalue (Class|KismetSystemLibrary|MakeLiteralInteger 20))
  (bind _returnvalue_2 (/ SizeY 2))
  (bind _returnvalue_3 (/ SizeX 2))
  (bind _returnvalue_4 (/ _returnvalue 2))
  (bind _returnvalue_5 (Math|Conversions|ToFloat(Integer) _returnvalue_3))
  (bind _returnvalue_6 (Math|Conversions|ToFloat(Integer) _returnvalue_2))
  (bind _returnvalue_7 (Math|Conversions|ToFloat(Integer) _returnvalue_4))
  (HUD|DrawRect "(R=1.000000,G=1.000000,B=1.000000,A=1.000000)" (- _returnvalue_5 _returnvalue_7) (- _returnvalue_6 1.0) (Math|Conversions|ToFloat(Integer) _returnvalue) 2.0)
  (HUD|DrawRect "(R=1.000000,G=1.000000,B=1.000000,A=1.000000)" (- _returnvalue_5 1.0) (- _returnvalue_6 _returnvalue_7) 2.0 (Math|Conversions|ToFloat(Integer) _returnvalue)))

(fn ConstructionScript)